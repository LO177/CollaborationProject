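; Rifle projectile actor that flies horizontally along the world X axis once fired.
; FiringSetup takes a Right or Left facing, sets a positive or negative speed, and calls StartTick to open a gate on Tick.
; Each tick then moves the actor by that fixed step without sweep or delta-time scaling, so speed depends on frame rate.
; It contains no active hit handling or destroy logic.
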(event Custom|Start%20Tick
  (Utilities|FlowControl|Gate true) ; enters at Open
)

(event EventTick
  (params (DeltaSeconds :type Float%20%28single-precision%29))
  (Utilities|FlowControl|Gate true
    (:Exit
      (bind _output_get (Variables|Default|SetReturnVector (+ (Transformation|GetActorLocation) (Math|Vector|MakeVector (Variables|Default|GetspeedProj) 0.0 0.0))))
      (Transformation|SetActorLocation _output_get false false))))

(event Collision|EventActorBeginOverlap
  (params (OtherActor :type Actor%20Object%20Reference)))

(event EventBeginPlay)

(event EventFiringSetup
  (params (directionFace :type String))
  (bind _output_get (Variables|Default|SetcasterDirection directionFace))
  (switch string _output_get
    (:Right
      (Variables|Default|SetspeedProj 5e+01))
    (:Left
      (Variables|Default|SetspeedProj -5e+01)))
  (CallFunction|StartTick))

(fn ConstructionScript)