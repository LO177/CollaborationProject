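; Rifle weapon actor that enables player input on BeginPlay and fires when Space Bar is pressed.
; While AmmoAttribute is above zero, it spawns a ProjectileRifle at the player character's transform and passes the weapon's direction and angle to its FiringSetup; otherwise it prints "Empty".
; Ammo decrement, AttachWeapon and FireWeapon nodes are left unwired, so firing does not reduce ammo in this graph.
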(event Collision|EventActorBeginOverlap
  (params (OtherActor :type Actor%20Object%20Reference)))

(event EventBeginPlay
  (Input|EnableInput (Game|GetPlayerController 0)))

(event Input|KeyboardEvents|SpaceBar
  (params (Key :type Key%20Structure))
  (:Pressed
    (if (> (Variables|Default|GetammoAttribute) 0)
      (bind _returnvalue (Game|SpawnActorfromClass "/Game/blueprints/ProjectileRifle.ProjectileRifle_C" (Transformation|GetActorTransform (Game|GetPlayerCharacter 0)) "Undefined" 0 0))
      (Class|ProjectileBase|FiringSetup _returnvalue (Variables|Default|GetdirectionWeap) (Variables|Default|GetdirectProj))
      (else
        (Development|PrintString "Empty")))))

(fn ConstructionScript)