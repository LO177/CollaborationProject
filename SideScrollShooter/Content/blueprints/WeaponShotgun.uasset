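; Shotgun weapon Blueprint that fires a spread of five projectiles when Space is pressed and ammo is above zero, otherwise printing an empty message.
; A loop spawns ProjectileShotgun actors at the player character's transform, passing each the weapon direction and a stepped angle through FiringSetup.
; Input enabling, attachment and ammo decrement logic are left unconnected, so firing does not consume ammo here.
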(event Collision|EventActorBeginOverlap
  (params (OtherActor :type Actor%20Object%20Reference)))

(event EventBeginPlay)

(event Input|KeyboardEvents|SpaceBar
  (params (Key :type Key%20Structure))
  (:Pressed
    (if (> (Variables|Default|GetammoAttribute) 0)
      (Development|PrintString "Weapon fired")
      (Variables|Default|SetdirectProj 40)
      (for _index (range 1 5)
        (bind _output_get (Variables|Default|SetdirectProj (+ (Variables|Default|GetdirectProj) 25)))
        (bind _returnvalue (Game|SpawnActorfromClass "/Game/blueprints/ProjectileShotgun.ProjectileShotgun_C" (Transformation|GetActorTransform (Game|GetPlayerCharacter 0)) "Undefined" 0 0))
        (Class|ProjectileBase|FiringSetup _returnvalue (Variables|Default|GetdirectionWeap) _output_get))
      (else
        (Development|PrintString "Empty")))))

(fn ConstructionScript)